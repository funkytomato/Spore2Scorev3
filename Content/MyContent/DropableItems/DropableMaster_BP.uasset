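; DropableMaster_BP is the master Blueprint for dropped items such as spores or mushrooms that link nearby life to the Mysellium trail.
; BeginPlay caches the Mysellium actor and starts a one-shot timer that marks the item mature.
; On maturing, it flags InteractableMaster_BP actors overlapping its sphere of influence as connected to the trail, with debug prints.
; An Illuminate event toggles its point light's visibility.
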(event Custom|UpdateLifeConnected
  ;[1 1 1] Connect Vegetation and Rocks within proximity to the Mysellium Trail
  ;;[1 1 1] Connect Life to Mysellium when Spore/Mushroom Matured
  (Variables|Default|SetIsMature true)
  (bind _output_get (Variables|Default|SetConnectedActors (Collision|GetOverlappingActors (Variables|Default|GetMyselliumSphereOfInfluence) "/Game/MyContent/Environment/InteractableItems/InteractableMaster_BP.InteractableMaster_BP_C" :!class /Script/Engine.PrimitiveComponent)))
  (for _array_element _output_get
    (bind _asinteractable_master_bp (Utilities|Casting|CastToInteractableMaster_BP _array_element))
    (Variables|/Game/MyContent/Environment/InteractableItems/InteractableMaster_BP.InteractableMaster_BP_C|SetConnectedToMyselliumTrail _asinteractable_master_bp true)
    (Development|PrintString (Utilities|GetDisplayName _asinteractable_master_bp)))
  (Development|PrintString "Update Life Connected"))

(event Custom|Illuminate
  (params (IsOn :type Boolean))
  (bind _pointlight (Variables|Default|GetPointLight))
  ;[1 1 1] Illuminate/Unilluminate
  (if IsOn
    (Rendering|SetVisibility _pointlight true false)
    (else
      (Rendering|SetVisibility _pointlight false false))))

(event EventBeginPlay
  ;[1 1 1] Connect Vegetation and Rocks within proximity to the Mysellium Trail
  (bind _returnvalue (Actor|GetActorOfClass "/Game/MyContent/Environment/Mysellium/Mysellium_BP.Mysellium_BP_C"))
  (Variables|Default|SetMysellium_Ref _returnvalue)
  (Variables|Default|SetIsMature false)
  (Utilities|Time|SetTimerbyEvent (delegate Custom|UpdateLifeConnected) 1.0 false 2.0))

(fn ConstructionScript)