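; PlantLifeMaster_BP is a plant actor, named as a master Blueprint, that simulates nutrients, health and growth.
; A looping one-second LifeCycle timer, rather than Tick, raises or drains nutrients depending on the Mycellium connection.
; High nutrients restore health and scale up the mesh, while depletion drains health, which drives dying and dead flags.
; BeginPlay also gives its PlantWidget_BP an owner reference; the Shrink branch is left unconnected.
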(event Custom|LifeCycle
  (bind _health (Variables|Health|GetHealth))
  (Utilities|FlowControl|Sequence
    (:then_0
      ;[1 1 1] Increase nutrients if connected to Mycellium
      (if (Variables|Default|GetMycelliumConnected)
        (CallFunction|IncreaseNutrients 5.0)
        (else
          (CallFunction|DecreaseNutrients 5.0))))
    (:then_1
      ;[1 1 1] Grow plant if nutrient level high
      (if (> (Variables|Health|GetNutrients) 1e+02)
        (CallFunction|Grow)))
    (:then_2
      ;[1 1 1] Plant is dying
      (if (and (> (Variables|Default|GetoldHealth) _health) (< _health (Variables|Default|GetLowHealth)))
        (Variables|Default|SetIsDying true)
        (else
          (Variables|Default|SetIsDying false)))
      (Variables|Default|SetoldHealth (Variables|Health|GetHealth)))
    (:then_3
      ;[1 1 1] Plant is dead
      (if (not (> (Variables|Health|GetHealth) 0.0))
        (Variables|Default|SetIsDead true)))))

(event Custom|AddWidget
  ;[1 1 1] Get reference to Widget_BP
  (bind _asplant_widget_bp (Utilities|Casting|CastToPlantWidget_BP (UserInterface|GetUserWidgetObject (Variables|Default|GetWidget))))
  (bind _output_get (Variables|Default|SetPlantWidget _asplant_widget_bp))
  (Variables|/Game/MyContent/Widgets/PlantWidget_BP.PlantWidget_BP_C|SetOwner _output_get self))

(event EventBeginPlay
  ;[1 1 1] Beginplay - Start LifeCycle timer and assign Plant Widget
  (|CallParentFunction)
  (Utilities|Time|SetTimerbyFunctionName 0 "LifeCycle" 1.0 true)
  (CallFunction|AddWidget))

(event Collision|EventActorBeginOverlap
  (params (OtherActor :type Actor%20Object%20Reference))
  (|CallParentFunction OtherActor) ; This node is disabled and will not be called.\nDrag off pins to build functionality.
)

(event EventTick
  (params (DeltaSeconds :type Float%20%28single-precision%29))
  (|CallParentFunction DeltaSeconds) ; This node is disabled and will not be called.\nDrag off pins to build functionality.
)

(fn ConstructionScript
  (|CallParentFunction))

(fn IncreaseNutrients
  (params (amount :type Float%20%28single-precision%29))
  (bind _output_get (Variables|Health|SetNutrients (Math|Float|Clamp(Float) (+ (Variables|Health|GetNutrients) amount) 0.0 (Variables|Health|GetMaxNutrients))))
  (Variables|Default|SetNutrientDepleted false)
  (if (> _output_get 8e+01)
    (CallFunction|IncreaseHealth 5.0)))

(fn DecreaseNutrients
  (params (amount :type Float%20%28single-precision%29))
  (bind _output_get (Variables|Health|SetNutrients (Math|Float|Clamp(Float) (- (Variables|Health|GetNutrients) amount) 0.0 (Variables|Health|GetMaxNutrients))))
  (if (not (> _output_get 0.0))
    (Variables|Default|SetNutrientDepleted true)
    (CallFunction|DecreaseHealth 5.0)))

(fn Grow
  (bind _staticmesh (Variables|Default|GetStaticMesh))
  (bind _basescale (Variables|Growth|GetBaseScale))
  (bind _returnvalue (Transformation|GetWorldScale _staticmesh))
  (Transformation|SetWorldScale3D _staticmesh (Math|Vector|MakeVector (+ (.x _returnvalue) _basescale) (+ (.y _returnvalue) _basescale) (+ (.z _returnvalue) (Variables|Growth|GetVerticalScale)))))

(fn Shrink
  (bind _staticmesh (Variables|Default|GetStaticMesh))
  (bind _basescale (Variables|Growth|GetBaseScale))
  (bind _returnvalue (Transformation|GetWorldScale _staticmesh))
  (Transformation|SetWorldScale3D _staticmesh (Math|Vector|MakeVector (- (.x _returnvalue) _basescale) (- (.y _returnvalue) _basescale) (- (.z _returnvalue) (Variables|Growth|GetVerticalScale)))))

(fn IncreaseHealth
  (params (amount :type Float%20%28single-precision%29))
  (Variables|Health|SetHealth (Math|Float|Clamp(Float) (+ (Variables|Health|GetHealth) amount) 0.0 (Variables|Health|GetMaxHealth))))

(fn DecreaseHealth
  (params (amount :type Float%20%28single-precision%29))
  (Variables|Health|SetHealth (Math|Float|Clamp(Float) (- (Variables|Health|GetHealth) amount) 0.0 (Variables|Health|GetMaxHealth))))