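; LevelItemMaster_BP is a level item actor, apparently a master class, that shows a widget when the player comes near.
; Overlaps on InteractionSphereOfInfluence with a ThirdPersonCharacter show the widget on entry and hide it on exit.
; On entry, RotateWidgettofacePlayer turns the widget toward player 0's follow camera using FindLookAtRotation.
; The rotation is set once per entry, as Tick is unused.
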(event OnComponentBeginOverlap(InteractionSphereOfInfluence)
  (params (OverlappedComponent :type Primitive%20Component%20Object%20Reference) (OtherActor :type Actor%20Object%20Reference) (OtherComp :type Primitive%20Component%20Object%20Reference) (OtherBodyIndex :type Integer) (bFromSweep :type Boolean) (SweepResult :type Hit%20Result%20Structure%20%28by%20ref%29))
  ;[1 1 1] Show/Don't Show Plant Widget
  (Utilities|Casting|CastToThirdPersonCharacter OtherActor)
  (CallFunction|RotateWidgettoFacePlayer)
  (Rendering|SetVisibility (Variables|Default|GetWidget) true false))

(event OnComponentEndOverlap(InteractionSphereOfInfluence)
  (params (OverlappedComponent :type Primitive%20Component%20Object%20Reference) (OtherActor :type Actor%20Object%20Reference) (OtherComp :type Primitive%20Component%20Object%20Reference) (OtherBodyIndex :type Integer))
  ;[1 1 1] Show/Don't Show Plant Widget
  (Utilities|Casting|CastToThirdPersonCharacter OtherActor)
  (Rendering|SetVisibility (Variables|Default|GetWidget) false false))

(event Custom|Rotate%20Widget%20to%20face%20Player
  ;[1 1 1] Rotate Widget to face Player
  (bind _asthird_person_character (Utilities|Casting|CastToThirdPersonCharacter (Game|GetPlayerCharacter 0)))
  (Transformation|SetWorldRotation (Variables|Default|GetWidget) (Math|Rotator|FindLookatRotation (Transformation|GetWorldLocation (Variables|Default|GetDefaultSceneRoot)) (Transformation|GetWorldLocation (Variables|/Game/ThirdPersonBP/Blueprints/ThirdPersonCharacter.ThirdPersonCharacter_C|GetFollowCamera _asthird_person_character))) false false))

(event EventBeginPlay)

(event Collision|EventActorBeginOverlap
  (params (OtherActor :type Actor%20Object%20Reference)))

(event EventTick
  (params (DeltaSeconds :type Float%20%28single-precision%29)))

(fn ConstructionScript)