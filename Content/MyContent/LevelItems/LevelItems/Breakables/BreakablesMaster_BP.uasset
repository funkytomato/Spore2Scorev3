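; BreakablesMaster_BP is a breakable level item, named as a master Blueprint, that degrades by losing nutrients and then disappears.
; BeginPlay starts a looping one-second timer that calls the Degrade event.
; Degrade subtracts MaxNutrients from Nutrients, clamps the result between zero and MaxNutrients, and destroys the actor at zero.
; Because each step subtracts the full maximum, any value up to that maximum is depleted in one call.
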(event Custom|Degrade
  ;[1 1 1] Degrade Item
  (bind _output_get (Variables|Default|SetNutrients (Math|Float|Clamp(Float) (- (Variables|Default|GetNutrients) (Variables|Default|GetMaxNutrients)) 0.0 (Variables|Default|GetMaxNutrients))))
  ;[1 1 1] Destroy once nutrients have been depleted
  (if (not (> _output_get 0.0))
    (Actor|DestroyActor)))

(event EventBeginPlay
  (|CallParentFunction)
  (Utilities|Time|SetTimerbyFunctionName 0 "Degrade" 1.0 true))

(event Collision|EventActorBeginOverlap
  (params (OtherActor :type Actor%20Object%20Reference))
  (|CallParentFunction OtherActor) ; This node is disabled and will not be called.\nDrag off pins to build functionality.
)

(event EventTick
  (params (DeltaSeconds :type Float%20%28single-precision%29))
  (|CallParentFunction DeltaSeconds) ; This node is disabled and will not be called.\nDrag off pins to build functionality.
)

(fn ConstructionScript
  (|CallParentFunction))