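; Master Blueprint for trees, extending a parent life cycle with death, decay and removal.
; On death, a one-time swap clears the static mesh, adds a destructible component at its transform and refills nutrients as dead wood.
; Each life cycle call on a dead tree drains nutrients, destroying the actor once they are depleted during decay.
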(event Custom|DeadTree
  (bind _staticmesh (Variables|Default|GetStaticMesh))
  ;[1 1 1] Display Dead Tree
  (Utilities|FlowControl|DoOnce false
    (:Completed
      (Components|StaticMesh|SetStaticMesh _staticmesh 0)
      (AddComponent|AddDestructibleComponent false (Transformation|GetRelativeTransform _staticmesh))
      (Variables|Default|SetIsDecaying true)
      ;[1 1 1] Set nutrient level back to 100% because has become new source of nutrients (dead wood)
      (CallFunction|IncreaseNutrients (Variables|Default|GetMaxNutrients)))))

(event Custom|DeadVisuals
  ;[1 1 1] Update visuals respectively to health
  (if (Variables|Default|GetIsDead)
    (CallFunction|DeadTree)))

(event EventBeginPlay
  (|CallParentFunction))

(event Collision|EventActorBeginOverlap
  (params (OtherActor :type Actor%20Object%20Reference))
  (|CallParentFunction OtherActor) ; This node is disabled and will not be called.\nDrag off pins to build functionality.
)

(event EventTick
  (params (DeltaSeconds :type Float%20%28single-precision%29))
  (|CallParentFunction DeltaSeconds) ; This node is disabled and will not be called.\nDrag off pins to build functionality.
)

(event EventLifeCycle
  ;[1 1 1] Tree Life Cycle
  (|CallParentFunction)
  (CallFunction|DeadVisuals)
  ;[1 1 1] Dead, decay item
  (if (Variables|Default|GetIsDead)
    (CallFunction|DecreaseNutrients 5.0)
    ;[1 1 1] Item is decaying, destroy when decayed
    (if (Variables|Default|GetIsDecaying)
      (if (Variables|Default|GetNutrientDepleted)
        (Actor|DestroyActor)))))

(fn ConstructionScript
  (|CallParentFunction))