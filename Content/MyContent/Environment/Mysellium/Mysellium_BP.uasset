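; Mysellium actor that models the level's fungal network, tracking connected life, nutrients, health and death.
; Bound messages add or remove life and move nutrients in or out, with drained nutrients passing into health changes.
; A looping timer opens the game instance's level complete or failed menu and resets per-cycle nutrient totals.
; Trail events toggle illumination on connected life and dim or restore the directional light.
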(event Custom|MyselliumLifeCycleTick
  ;[1 1 1] Mysellium Tick Event
  ;;[1 1 1] Check Player Success/Failure
  (CallFunction|CheckLevelSuccess)
  (CallFunction|CheckLevelFailed)
  (Variables|Nutrients|SetNutrientOutput 0.0)
  (Variables|Nutrients|SetNutrientInput 0.0))

(event Custom|IlluminateMyselliumTrail
  ;[1 1 1] Mysellium Trail Illumination
  (for _array_element (Variables|Mysellium|GetMyselliumLife)
    (bind _asdropable_master_bp (Utilities|Casting|CastToDropableMaster_BP _array_element)
      (:then
        (Default|Illuminate _asdropable_master_bp true))
      (:CastFailed
        (bind _asinteractable_master_bp (Utilities|Casting|CastToInteractableMaster_BP _array_element))
        (Default|Illuminate _asinteractable_master_bp))))
  (CallFunction|DarkentheWorld))

(event Custom|CheckLevelFailed
  ;[1 1 1] Check if Level Failed, Show Level Failed Menu
  (if (Variables|Health|GetIsDead)
    (bind _asspore_2score_game_instance (Utilities|Casting|CastToSpore2ScoreGameInstance (Game|GetGameInstance)))
    (Default|ShowLevelFailedMenu _asspore_2score_game_instance)))

(event Custom|ResetLevelValues
  ;[1 1 1] Reset Level Properties
  (Variables|Health|SetHealth 1e+02)
  (Variables|Nutrients|SetNutrients (Variables|Nutrients|GetInitialNutrientLevel))
  (Variables|Game|SetLifeCount 0))

(event Custom|Remove%20Life%20From%20Mysellium_Event
  (params (Life%20To%20Remove :type Actor%20Object%20Reference))
  ;[1 1 1] Initialise and configure Messages
  ;;[1 1 1] Update Mysellium Life
  (CallFunction|RemoveLifefromMysellium Life%20To%20Remove))

(event Custom|UnIlluminateMySelliumTrail
  ;[1 1 1] Mysellium Trail Illumination
  (for _array_element (Variables|Mysellium|GetMyselliumLife)
    (bind _asdropable_master_bp (Utilities|Casting|CastToDropableMaster_BP _array_element)
      (:then
        (Default|Illuminate _asdropable_master_bp false))
      (:CastFailed
        (bind _asinteractable_master_bp (Utilities|Casting|CastToInteractableMaster_BP _array_element))
        (Default|Illuminate _asinteractable_master_bp))))
  (CallFunction|BrightentheWorld))

(event Custom|DarkenTheWorld
  ;[1 1 1] World Illumination
  (bind _returnvalue (Actor|GetActorOfClass "/Script/Engine.DirectionalLight"))
  (Rendering|Components|Light|SetIntensity (Variables|/Script/Engine.Light|GetLightComponent _returnvalue) 0.0))

(event Custom|AddLifeToMysellium_Event
  (params (NewLifeToAdd :type Actor%20Object%20Reference))
  ;[1 1 1] Initialise and configure Messages
  ;;[1 1 1] Update Mysellium Life
  (CallFunction|AddLifetoMysellium NewLifeToAdd))

(event Custom|Recieve%20Nutrients_Event
  (params (Amount :type Float%20%28single-precision%29))
  ;[1 1 1] Initialise and configure Messages
  ;;[1 1 1] Recieve Nutrients from Life
  (Development|PrintString (Utilities|String|ToString(Float) Amount))
  (Development|PrintString "Increase Nutrients Recieved")
  (CallFunction|IncreaseNutrientReceivedAmount Amount)
  (CallFunction|IncreaseNutrients Amount))

(event Custom|DecreaseNutrientsMessage_Event
  (params (Amount :type Float%20%28single-precision%29))
  ;[1 1 1] Initialise and configure Messages
  ;;[1 1 1] Nutrients Sent to Life
  (Development|PrintString (Utilities|String|ToString(Float) Amount))
  (Development|PrintString "Increase Nutrients Sent")
  (CallFunction|IncreaseNutrientsSentAmount Amount)
  (CallFunction|DecreaseNutrients Amount))

(event Custom|BrightenTheWorld
  ;[1 1 1] World Illumination
  (bind _returnvalue (Actor|GetActorOfClass "/Script/Engine.DirectionalLight"))
  (Rendering|Components|Light|SetIntensity (Variables|/Script/Engine.Light|GetLightComponent _returnvalue) 1e+01))

(event Custom|CheckLevelSuccess
  ;[1 1 1] Show Level Complete Menu
  (if (> (Utilities|Array|Length (Variables|Mysellium|GetMyselliumLife)) (Variables|Game|GetLifeformWinCount))
    (if (>= (Variables|Nutrients|GetNutrients) 1e+02)
      (bind _asspore_2score_game_instance (Utilities|Casting|CastToSpore2ScoreGameInstance (Game|GetGameInstance)))
      (Default|ShowLevelCompleteMenu _asspore_2score_game_instance))))

(event Custom|AddWidget
  ;[1 1 1] BeginPlay - Get reference to Widget_BP
  (bind _asmysellium_widget_bp (Utilities|Casting|CastToMyselliumWidget_BP (UserInterface|GetUserWidgetObject (Variables|Default|GetWidget))))
  (bind _output_get (Variables|Widgets|SetMyselliumWidget _asmysellium_widget_bp))
  (Variables|/Game/MyContent/Widgets/MyselliumWidget_BP.MyselliumWidget_BP_C|SetOwningActor _output_get self))

(event EventBeginPlay
  ;[1 1 1] Initialise and configure Messages
  (EventDispatchers|BindEventtoAddLifetoMyselliumMessage (delegate Custom|AddLifeToMysellium_Event))
  (EventDispatchers|BindEventtoRemoveLifefromMyselliumMessage (delegate Custom|Remove%20Life%20From%20Mysellium_Event))
  (EventDispatchers|BindEventtoIncreaseNutrientsMessage (delegate Custom|Recieve%20Nutrients_Event))
  (EventDispatchers|BindEventtoDecreaseNutrientsMessage (delegate Custom|DecreaseNutrientsMessage_Event))
  ;[1 1 1] Mysellium Tick Event
  (Utilities|Time|SetTimerbyEvent (delegate Custom|MyselliumLifeCycleTick) 0.75 true))

(fn ConstructionScript)

(fn PopulateMyselliumLife)

(fn IncreaseNutrientReceivedAmount
  (params (NutrientAmount :type Float%20%28single-precision%29))
  (bind _output_get (Variables|Nutrients|SetNutrientInput (+ (Variables|Nutrients|GetNutrientInput) NutrientAmount)))
  (Variables|Mysellium|SetMNReceivedThisCycle _output_get)
  (return))

(fn CheckHealth
  (if (< (Variables|Nutrients|GetNutrients) 1e+01)
    (Variables|Health|SetHealth (Math|Float|Clamp(Float) (- (Variables|Health|GetHealth) 1.0) 0.0 1e+02))))

(fn AddLifetoMysellium
  (params (NewItem :type Actor%20Object%20Reference%20%28by%20ref%29))
  (bind _asinteractable_master_bp (Utilities|Casting|CastToInteractableMaster_BP NewItem)
    (:then
      (Variables|/Game/MyContent/Environment/InteractableItems/InteractableMaster_BP.InteractableMaster_BP_C|SetConnectedToMyselliumTrail _asinteractable_master_bp true)
      (Utilities|Array|AddUnique (Variables|Mysellium|GetMyselliumLife) NewItem)
      (Variables|Game|SetLifeCount (+ (Variables|Game|GetLifeCount) 1)))
    (:CastFailed
      (Development|PrintString "Failed to cast to InteractableMaster in Mysellium Add Life"))))

(fn RemoveLifefromMysellium
  (params (Item :type Actor%20Object%20Reference%20%28by%20ref%29))
  (bind _asinteractable_master_bp (Utilities|Casting|CastToInteractableMaster_BP Item))
  (Variables|/Game/MyContent/Environment/InteractableItems/InteractableMaster_BP.InteractableMaster_BP_C|SetConnectedToMyselliumTrail _asinteractable_master_bp false)
  (Utilities|Array|RemoveItem (Variables|Mysellium|GetMyselliumLife) Item)
  (Variables|Game|SetLifeCount (- (Variables|Game|GetLifeCount) 1)))

(fn IncreaseNutrients
  (params (amount :type Float%20%28single-precision%29))
  (Variables|Nutrients|SetNutrients (Math|Float|Clamp(Float) (+ amount (Variables|Nutrients|GetNutrients)) 0.0 (Variables|Nutrients|GetMaxNutrients)))
  (return))

(fn DecreaseNutrients
  (params (amount :type Float%20%28single-precision%29))
  (bind _output_get (Variables|Nutrients|SetNutrients (Math|Float|Clamp(Float) (- (Variables|Nutrients|GetNutrients) amount) 0.0 (Variables|Nutrients|GetMaxNutrients))))
  (if (<= _output_get 0.0)
    (CallFunction|DecreaseHealth amount)
    (return)))

(fn IncreaseHealth
  (params (Amount :type Float%20%28single-precision%29))
  (Variables|Health|SetHealth (Math|Float|Clamp(Float) (+ Amount (Variables|Health|GetHealth)) 0.0 (Variables|Health|GetMaxHealth))))

(fn DecreaseHealth
  (params (Amount :type Float%20%28single-precision%29))
  (bind _output_get (Variables|Health|SetHealth (Math|Float|Clamp(Float) (- Amount (Variables|Health|GetHealth)) 0.0 (Variables|Health|GetMaxHealth))))
  (if (not (> _output_get 0.0))
    (Variables|Health|SetIsDead true)))

(fn IncreaseNutrientsSentAmount
  (params (amount :type Float%20%28single-precision%29))
  (Variables|Nutrients|SetNutrientOutput (+ (Variables|Nutrients|GetNutrientOutput) amount))
  (return))