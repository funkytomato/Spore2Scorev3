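; Master Blueprint for interactable trees with leaves that reflect their health and share nutrients with nearby plant life.
; A one-second timer lights the tree when connected to a mycelium trail and shows or hides leaves at a low-health threshold, calling empty grow and fall hooks.
; A second timer, while the tree flourishes, takes nutrients from flourishing biological actors in its mycelium sphere and gives them to struggling ones.
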(event EventBeginPlay
  (|CallParentFunction)
  (Utilities|Time|SetTimerbyFunctionName 0 "Update Visual Representation to Health" 1.0 true)
  (Utilities|Time|SetTimerbyFunctionName 0 "Support Life Cycle" 1.0 true))

(event Collision|EventActorBeginOverlap
  (params (OtherActor :type Actor%20Object%20Reference))
  (|CallParentFunction OtherActor) ; This node is disabled and will not be called.\nDrag off pins to build functionality.
)

(event EventTick
  (params (DeltaSeconds :type Float%20%28single-precision%29))
  (|CallParentFunction DeltaSeconds) ; This node is disabled and will not be called.\nDrag off pins to build functionality.
)

(fn ConstructionScript
  (|CallParentFunction))

(fn UpdateVisualRepresentationtoHealth
  (bind _leaves (Variables|Default|GetLeaves))
  (bind _illuminationlight (Variables|Default|GetIlluminationLight))
  ;[1 1 1] Illuminate If connected to Mysellium
  (if (Variables|Default|GetConnectedToMyselliumTrail)
    (Rendering|SetVisibility _illuminationlight true false)
    (else
      (Rendering|SetVisibility _illuminationlight false false)))
  ;[1 1 1] Show/Not Show Leaves according to health
  (if (<= (Variables|Default|GetHealth) (Variables|Default|GetLowHealthValue))
    (Rendering|SetVisibility _leaves false false)
    (CallFunction|LeavesFall)
    (else
      (Rendering|SetVisibility _leaves true false)
      (CallFunction|GrowLeaves))))

(fn GrowLeaves)

(fn LeavesFall)

(fn SupportLifeCycle
  (bind _myselliumhealthbonus (Variables|Default|GetMySelliumHealthBonus))
  ;[1 1 1] Calculate how many nutrients can be sent to supported local life
  (bind _isflourishing (CallFunction|IsFlourishing))
  (if _isflourishing
    (for _array_element (Collision|GetOverlappingActors (Variables|Default|GetMyselliumSphereOfInfluence) "/Game/MyContent/Environment/InteractableItems/Biological/BiologicalMaster_BP.BiologicalMaster_BP_C" :!class /Script/Engine.PrimitiveComponent)
      (bind _asbiological_master_bp (Utilities|Casting|CastToBiologicalMaster_BP _array_element))
      (bind _isflourishing_2 (Default|IsFlourishing _asbiological_master_bp))
      (if _isflourishing_2
        ;;[1 1 1] Consume nutrients from plant life nearby
        (Default|CallDecreaseNutrientsMessage _asbiological_master_bp _myselliumhealthbonus)
        (CallFunction|IncreaseNutrients _myselliumhealthbonus)
        (else
          ;;[1 1 1] Provide Nutrients to plant life nearby
          (Default|CallIncreaseNutrientsMessage _asbiological_master_bp _myselliumhealthbonus)
          (CallFunction|DecreaseNutrients _myselliumhealthbonus))))))