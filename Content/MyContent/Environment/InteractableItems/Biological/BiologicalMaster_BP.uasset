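; BiologicalMaster_BP is a biological interactable item, apparently a master class, that runs a plant health and nutrient life cycle.
; A looping timer drives LifeCycle, which derives flourishing from health and nutrients and calculates surplus nutrients to send to Mysellium.
; When decayable and decaying, it spawns a NutrientDeposit_BP holding its nutrients and destroys itself.
; The dying leaf-browning and dead-mesh steps are empty stubs.
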(event EventBeginPlay
  (|CallParentFunction)
  ;[1 1 1] Start on Plant Health Cycle tick
  (Utilities|Time|SetTimerbyFunctionName 0 "LifeCycle" 1.0 true))

(fn ConstructionScript
  (|CallParentFunction))

(fn LifeCycle
  (bind _flourishingnutrientvalue (Variables|Default|GetFlourishingNutrientValue))
  (bind _nutrients (Variables|Default|GetNutrients))
  (Utilities|FlowControl|Sequence
    (:then_0
      ;[1 1 1] Reset variables for start of cycle
      (Variables|Default|SetMyselliumNutrientAmountToSend 0.0)
      (CallFunction|AmIFlourishing))
    (:then_1
      ;[1 1 1] Calculate how many nutrients can be sent to Mysellium
      (if (Variables|Default|GetIsFlourishing)
        ;;[1 1 1] Calculate excessive nutrients
        (if (< _nutrients _flourishingnutrientvalue)
          (Variables|Default|SetMyselliumNutrientAmountToSend 0.0)
          (else
            (bind _output_get (Variables|Default|SetMyselliumNutrientAmountToSend (- _nutrients _flourishingnutrientvalue)))))))
    (:then_2
      ;[1 1 1] IsDying, brown leaves
      (if (Variables|Default|GetIsDying)
        (CallFunction|BrownLeaves)))
    (:then_3
      ;[1 1 1] Is Dead, show dead mesh
      (if (Variables|Default|GetIsDead)
        (Utilities|FlowControl|DoOnce false)))
    (:then_4
      ;[1 1 1] IsDecaying, spawn a nutrient deposit (need a different check for debris and carcass etc.)
      (if (Variables|Default|GetIsDecayable)
        (if (Variables|Default|GetIsDecaying)
          (bind _returnvalue (Game|SpawnActorfromClass "/Game/MyContent/Environment/Deposits/NutrientDeposit_BP.NutrientDeposit_BP_C" (Transformation|GetWorldTransform (Variables|Default|GetStaticMesh)) "AlwaysSpawn" 0 0))
          (Variables|/Game/MyContent/Environment/Deposits/NutrientDeposit_BP.NutrientDeposit_BP_C|SetNutrientStoreLevel _returnvalue (Math|Float|Truncate (Variables|Default|GetNutrients)))
          (Actor|DestroyActor))))))

(fn AmIFlourishing
  (bind _output_get (Variables|Default|SetIsFlourishing (and (> (Variables|Default|GetHealth) 99.0) (> (Variables|Default|GetNutrients) (Variables|Default|GetFlourishingNutrientValue)))))
  (return _output_get))

(fn BrownLeaves)