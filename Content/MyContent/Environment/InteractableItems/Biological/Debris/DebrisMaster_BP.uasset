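; DebrisMaster_BP is, by its name, the master Blueprint for biological debris items that can connect to a Mysellium trail.
; UpdateVisualHealthRepresentation shows the Mushrooms component while Health is above zero and the debris is connected to a trail, hiding it when unconnected.
; At zero or lower Health, it calls CallRemoveLifeFromMyselliumMessage on MyselliumRef, passing itself, then destroys itself.
; The event graph is empty apart from disabled default nodes.
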(event EventBeginPlay
  (|CallParentFunction) ; This node is disabled and will not be called.\nDrag off pins to build functionality.
)

(event Collision|EventActorBeginOverlap
  (params (OtherActor :type Actor%20Object%20Reference)))

(event EventTick
  (params (DeltaSeconds :type Float%20%28single-precision%29)))

(fn ConstructionScript
  (|CallParentFunction))

(fn UpdateVisualHealthRepresentation
  (bind _mushrooms (Variables|Default|GetMushrooms))
  (if (> (Variables|Default|GetHealth) 0.0)
    (if (Variables|Default|GetConnectedToMyselliumTrail)
      (Rendering|SetVisibility _mushrooms true false)
      (else
        (Rendering|SetVisibility _mushrooms false false)))
    (else
      (Default|CallRemoveLifefromMyselliumMessage (Variables|Default|GetMysellium_Ref) self)
      (Actor|DestroyActor))))