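; Large tree Blueprint, an interactable biological item that shows its health through foliage and growth.
; A looping one-second timer started on BeginPlay compares Health to LowHealthValue, hiding the Leaves at or below it and showing them otherwise.
; Above that threshold, full health also nudges the trunk mesh and leaves up in world scale each tick of the timer, with no upper limit.
; LeavesFall and GrowLeaves are empty placeholder events.
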(event Custom|UpdateVisualRespectiveToHealth
  (bind _leaves (Variables|Default|GetLeaves))
  ;[1 1 1] Show/Not Show Leaves according to health
  (if (<= (Variables|Default|GetHealth) (Variables|Default|GetLowHealthValue))
    (Rendering|SetVisibility _leaves false false)
    (CallFunction|LeavesFall)
    (else
      (Rendering|SetVisibility _leaves true false)
      (CallFunction|GrowLeaves)
      (if (>= (Variables|Default|GetHealth) 1e+02)
        (CallFunction|Grow)))))

(event Custom|Grow%20Leaves)

(event Custom|Leaves%20Fall)

(event Custom|Grow
  (bind _staticmesh (Variables|Default|GetStaticMesh))
  (Transformation|SetWorldScale3D _staticmesh (+ (Transformation|GetWorldScale _staticmesh) 0.001))
  (Transformation|SetWorldScale3D (Variables|Default|GetLeaves) (+ (Transformation|GetWorldScale (Variables|Default|GetLeaves)) 0.001)))

(event EventBeginPlay
  (|CallParentFunction)
  (Utilities|Time|SetTimerbyFunctionName 0 "UpdateVisualRespectiveToHealth" 1.0 true))

(fn ConstructionScript
  (|CallParentFunction))