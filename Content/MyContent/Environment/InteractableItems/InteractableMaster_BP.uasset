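; Base Blueprint for interactable environment items such as plants and rocks, tracking health, nutrients and pollution.
; Bound message events adjust these stats, with nutrient levels feeding health and zero health leading to death, then delayed decay.
; Player overlap shows a camera-facing health widget and refreshes a light that glows only when healthy and connected to the Mysellium trail.
; Interact only prints clean, smash or hug placeholders, and the sparkle effect is unused.
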(event OnComponentBeginOverlap(InteractionSphereOfInfluence)
  (params (OverlappedComponent :type Primitive%20Component%20Object%20Reference) (OtherActor :type Actor%20Object%20Reference) (OtherComp :type Primitive%20Component%20Object%20Reference) (OtherBodyIndex :type Integer) (bFromSweep :type Boolean) (SweepResult :type Hit%20Result%20Structure%20%28by%20ref%29))
  ;[1 1 1] Update Plant Illumination/Sparkle corresponding plant Health and show the Health widget
  (Utilities|Casting|CastToSpore2ScoreCharacter OtherActor)
  (CallFunction|UpdatePlantHealthVisual)
  (CallFunction|RotatetoFacePlayer)
  (Rendering|SetVisibility (Variables|Default|GetWidget) true false))

(event OnComponentEndOverlap(InteractionSphereOfInfluence)
  (params (OverlappedComponent :type Primitive%20Component%20Object%20Reference) (OtherActor :type Actor%20Object%20Reference) (OtherComp :type Primitive%20Component%20Object%20Reference) (OtherBodyIndex :type Integer))
  ;[1 1 1] Update Plant Illumination/Sparkle corresponding plant Health and show the Health widget
  (Utilities|Casting|CastToSpore2ScoreCharacter OtherActor)
  (CallFunction|UpdatePlantHealthVisual)
  (Rendering|SetVisibility (Variables|Default|GetWidget) false false))

(event Custom|RotateToFacePlayer
  ;[1 1 1] Rotate Widget to face Player
  (bind _asspore_2score_character (Utilities|Casting|CastToSpore2ScoreCharacter (Game|GetPlayerCharacter 0)))
  (Transformation|SetWorldRotation (Variables|Default|GetWidget) (Math|Rotator|FindLookatRotation (Transformation|GetWorldLocation (Variables|Default|GetDefaultSceneRoot)) (Transformation|GetWorldLocation (Variables|/Game/MyContent/Characters/Blueprints/Spore2ScoreCharacter.Spore2ScoreCharacter_C|GetFollowCamera _asspore_2score_character))) false false))

(event Custom|DecreaseHealth
  (params (DecreaseAmount :type Float%20%28single-precision%29))
  ;[1 1 1] Update Health Property
  (Variables|Health|SetHealth (Math|Float|Clamp(Float) (- (Variables|Health|GetHealth) DecreaseAmount) 0.0 (Variables|Health|GetMaxHealth)))
  (Variables|Default|SetIsDying true)
  (if (not (> (Variables|Health|GetHealth) 0.0))
    (Variables|Default|SetIsDead true)
    (Utilities|FlowControl|Delay 5.0)
    (Variables|Default|SetIsDecaying true)))

(event Custom|DecreaseHealthMessage_Event
  (params (Amount :type Float%20%28single-precision%29))
  ;[1 1 1] Boost Health from Mysellium
  (CallFunction|DecreaseHealth Amount))

(event Custom|IncreasePollutionMessage_Event
  (params (Amount :type Float%20%28single-precision%29))
  ;[1 1 1] Boost Health from Mysellium
  (CallFunction|IncreasePollution Amount))

(event Custom|DecreasePollutionMessage_Event
  (params (Amount :type Float%20%28single-precision%29))
  ;[1 1 1] Boost Health from Mysellium
  (CallFunction|DecreasePollution Amount))

(event Custom|ReceiveNutrients_Event
  (params (Amount :type Float%20%28single-precision%29))
  ;[1 1 1] Boost Health from Mysellium
  (CallFunction|IncreaseNutrients Amount)
  (Variables|Mysellium|SetMyselliumRecievedNutrientAmount Amount))

(event Custom|DecreasePollution
  (params (AmountToReduce :type Float%20%28single-precision%29))
  ;[1 1 1] Update Pollution Level
  (Variables|Pollution|SetPollutionLevel (- (Variables|Pollution|GetPollutionLevel) AmountToReduce)))

(event Custom|IncreasePollution
  (params (AmountToIncrease :type Float%20%28single-precision%29))
  ;[1 1 1] Update Pollution Level
  (Variables|Pollution|SetPollutionLevel (+ (Variables|Pollution|GetPollutionLevel) AmountToIncrease)))

(event Custom|IncreaseHealth
  (params (HealthAmount :type Float%20%28single-precision%29))
  ;[1 1 1] Update Health Property
  (if (< (Variables|Health|GetHealth) (Variables|Health|GetMaxHealth))
    (Variables|Health|SetHealth (Math|Float|Clamp(Float) (+ (Variables|Health|GetHealth) HealthAmount) 0.0 (Variables|Health|GetMaxHealth)))
    (Variables|Default|SetIsDying false)
    (if (> (Variables|Health|GetHealth) 0.0)
      (Variables|Default|SetIsDead false)
      (Variables|Default|SetIsDecaying false))))

(event Custom|IncreaseNutrients
  (params (amount :type Float%20%28single-precision%29))
  ;[1 1 1] Update Nutrients Property
  (Variables|Nutrients|SetNutrients (Math|Float|Clamp(Float) (+ (Variables|Nutrients|GetNutrients) amount) 0.0 (Variables|Nutrients|GetMaxNutrients)))
  (if (> (Variables|Nutrients|GetNutrients) 0.0)
    (Variables|Nutrients|SetIsNutrientDepleted false)
    (else
      (Variables|Nutrients|SetIsNutrientDepleted true)))
  (if (>= (Variables|Nutrients|GetNutrients) 1e+02)
    (CallFunction|IncreaseHealth amount)
    (else
      (Development|PrintString "Interactable Master:- Nutrients is not above 100"))))

(event Custom|DecreaseNutrients
  (params (amount :type Float%20%28single-precision%29))
  ;[1 1 1] Update Nutrients Property
  (Variables|Nutrients|SetNutrients (Math|Float|Clamp(Float) (- (Variables|Nutrients|GetNutrients) amount) 0.0 (Variables|Nutrients|GetMaxNutrients)))
  (if (> (Variables|Nutrients|GetNutrients) 0.0)
    (Variables|Nutrients|SetIsNutrientDepleted false)
    (else
      (Variables|Nutrients|SetIsNutrientDepleted true)
      (CallFunction|DecreaseHealth amount))))

(event Custom|DecreaseNutrientsMessage_Event
  (params (Amount :type Float%20%28single-precision%29))
  ;[1 1 1] Boost Health from Mysellium
  (CallFunction|DecreaseNutrients Amount))

(event Custom|IncreaseHealthMessage_Event
  (params (Amount :type Float%20%28single-precision%29))
  ;[1 1 1] Boost Health from Mysellium
  (CallFunction|IncreaseHealth Amount))

(event EventInteract
  ;[1 1 1] Interact with Game Items
  ;;[1 1 1] Cleanup Pollution
  (if (Variables|Pollution|GetPolluted)
    (Development|PrintString "Clean Pollution")
    (else
      ;;[1 1 1] Is a rock, smash it, to release minerals
      (if (Variables|Health|GetBreakable)
        (Development|PrintString "Smash Rock")
        (else
          ;;[1 1 1] Hug Tree, give some love
          (if (Variables|Health|GetHuggable)
            (Development|PrintString "Hug!!!")))))))

(event EventBeginPlay
  ;[1 1 1] Get reference to Mysellium BP
  (bind _returnvalue (Actor|GetActorOfClass "/Game/MyContent/Environment/Mysellium/Mysellium_BP.Mysellium_BP_C"))
  (Variables|Mysellium|SetMysellium_Ref _returnvalue)
  ;[1 1 1] Get Reference to Widget_BP
  (bind _asplant_widget_bp (Utilities|Casting|CastToPlantWidget_BP (UserInterface|GetUserWidgetObject (Variables|Default|GetWidget))))
  (bind _output_get (Variables|Default|SetHealthWidget _asplant_widget_bp))
  (Variables|/Game/MyContent/Widgets/PlantWidget_BP.PlantWidget_BP_C|SetOwner _output_get self)
  ;[1 1 1] Show the Plant's Health status on BeginPlay
  (CallFunction|UpdatePlantHealthVisual)
  ;[1 1 1] Boost Health from Mysellium
  (EventDispatchers|BindEventtoIncreaseNutrientsMessage (delegate Custom|ReceiveNutrients_Event))
  (EventDispatchers|BindEventtoDecreaseNutrientsMessage (delegate Custom|DecreaseNutrientsMessage_Event))
  (EventDispatchers|BindEventtoIncreaseHealthMessage (delegate Custom|IncreaseHealthMessage_Event))
  (EventDispatchers|BindEventtoDecreaseHealthMessage (delegate Custom|DecreaseHealthMessage_Event))
  (EventDispatchers|BindEventtoIncreasePollutionMessage (delegate Custom|IncreasePollutionMessage_Event))
  (EventDispatchers|BindEventtoDecreasePollutionMessage (delegate Custom|DecreasePollutionMessage_Event)))

(fn ConstructionScript)

(fn IsHealthy
  (return (>= (Variables|Health|GetHealth) (Variables|Health|GetLowHealthValue))))

(fn Illuminate
  (Rendering|SetVisibility (Variables|Default|GetIlluminationLight) true false))

(fn Sparkle
  (Development|PrintString "Make Tree Sparkle")
  (Components|Activation|SetActive (Variables|Default|GetSparkleParticles) false false))

(fn UpdatePlantHealthVisual
  ;[1 1 1] Make Plant Sparkle if healthy
  (bind _ishealthy (CallFunction|IsHealthy))
  (if (and _ishealthy (Variables|Mysellium|GetConnectedToMyselliumTrail))
    (CallFunction|Illuminate)
    (else
      (CallFunction|UnIlluminate))))

(fn UnIlluminate
  (Rendering|SetVisibility (Variables|Default|GetIlluminationLight) false false))

(fn ShowPollution
  (bind _pollutiondecal (Variables|Default|GetPollutionDecal))
  (if (Variables|Pollution|GetPolluted)
    (Rendering|SetVisibility _pollutiondecal true false)
    (else
      (Rendering|SetVisibility _pollutiondecal false false))))

(fn IsPolluted
  (bind _pollutionlevel (Variables|Pollution|GetPollutionLevel))
  (bind _highpollutionvalue (Variables|Pollution|GetHighPollutionValue))
  (bind _returnvalue (>= _pollutionlevel _highpollutionvalue))
  (if _returnvalue
    (Variables|Pollution|SetPolluted true)
    (else
      (Variables|Pollution|SetPolluted false)))
  (return _returnvalue))

(fn IsMaxHealth
  (return (>= (Variables|Health|GetHealth) 1e+02)))