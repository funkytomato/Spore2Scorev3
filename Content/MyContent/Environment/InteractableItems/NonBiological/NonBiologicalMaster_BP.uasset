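; Master Blueprint for non-biological decayable items that the mycelium breaks down for nutrients.
; BeginPlay caches the Mysellium actor, binds itself to its decay widget and starts a looping one-second degrade timer.
; While connected to a Mysellium trail and not depleted, each tick transfers nutrients to the Mysellium, faster if smashed.
; At zero nutrients it tells the Mysellium to remove it and self-destructs after a short lifespan.
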(event EventBeginPlay
  (Variables|Default|SetIsDecayable true)
  ;[1 1 1] Get reference to Mysellium BP
  (bind _returnvalue (Actor|GetActorOfClass "/Game/MyContent/Environment/Mysellium/Mysellium_BP.Mysellium_BP_C"))
  (Variables|Default|SetMysellium_Ref _returnvalue)
  ;[1 1 1] Get Reference to Widget_BP
  (bind _asdecayable_widget_bp (Utilities|Casting|CastToDecayableWidget_BP (UserInterface|GetUserWidgetObject (Variables|Default|GetWidget))))
  (bind _output_get (Variables|Default|SetDecayableWidget _asdecayable_widget_bp))
  (Variables|/Game/MyContent/Widgets/DecayableWidget_BP.DecayableWidget_BP_C|SetOwner _output_get self)
  ;[1 1 1] Show the Plant's Health status on BeginPlay
  (CallFunction|UpdatePlantHealthVisual)
  (Utilities|Time|SetTimerbyFunctionName 0 "Degrade Cycle" 1.0 true))

(fn ConstructionScript
  (|CallParentFunction))

(fn DegradeCycle
  (bind _mysellium_ref (Variables|Default|GetMysellium_Ref))
  ;[1 1 1] Check not nutrient depleted
  (if (not (Variables|Default|GetIsNutrientDepleted))
    ;[1 1 1] Check connected to Mysellium Trail
    (if (Variables|Default|GetConnectedToMyselliumTrail)
      ;[1 1 1] If smashed, send more nutrients, if not smashed recieve more mysellium to help break down
      (if (Variables|Default|GetIsSmashed)
        (Default|CallIncreaseNutrientsMessage _mysellium_ref 5.0)
        (CallFunction|DecreaseNutrients 5.0)
        (else
          (Default|CallIncreaseNutrientsMessage _mysellium_ref 1.0)
          (CallFunction|DecreaseNutrients 1.0)))
      (if (not (> (Variables|Default|GetNutrients) 0.0))
        (Default|CallRemoveLifefromMyselliumMessage (Variables|Default|GetMysellium_Ref) self)
        (Actor|SetLifeSpan 2.0)))))