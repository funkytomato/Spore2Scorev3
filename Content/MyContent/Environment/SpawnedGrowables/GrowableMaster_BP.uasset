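; Base Blueprint for a growable plant that gains or loses health with its nutrient level, grows while flourishing and is destroyed at zero health.
; A one-second looping LifeCycle timer drains nutrients while deteriorating, which costs health once depleted, and scales up the mesh when health and nutrients are high.
; Bound messages add nutrients or toggle deterioration.
; An interaction sphere shows the health widget, turned toward the player's camera on overlap.
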(event OnComponentBeginOverlap(InteractionSphereOfInfluence)
  (params (OverlappedComponent :type Primitive%20Component%20Object%20Reference) (OtherActor :type Actor%20Object%20Reference) (OtherComp :type Primitive%20Component%20Object%20Reference) (OtherBodyIndex :type Integer) (bFromSweep :type Boolean) (SweepResult :type Hit%20Result%20Structure%20%28by%20ref%29))
  ;[1 1 1] Show or Hide Widget if Player nearby
  (Utilities|Casting|CastToSpore2ScoreCharacter OtherActor)
  (CallFunction|RotatetoFacePlayer)
  (Rendering|SetVisibility (Variables|Default|GetWidget) true false))

(event OnComponentEndOverlap(InteractionSphereOfInfluence)
  (params (OverlappedComponent :type Primitive%20Component%20Object%20Reference) (OtherActor :type Actor%20Object%20Reference) (OtherComp :type Primitive%20Component%20Object%20Reference) (OtherBodyIndex :type Integer))
  ;[1 1 1] Show or Hide Widget if Player nearby
  (Utilities|Casting|CastToSpore2ScoreCharacter OtherActor)
  (Rendering|SetVisibility (Variables|Default|GetWidget) false false))

(event Custom|RotateToFacePlayer
  ;[1 1 1] Rotate Widget to face Player
  (bind _asspore_2score_character (Utilities|Casting|CastToSpore2ScoreCharacter (Game|GetPlayerCharacter 0)))
  (Transformation|SetWorldRotation (Variables|Default|GetWidget) (Math|Rotator|FindLookatRotation (Transformation|GetWorldLocation (Variables|Default|GetDefaultSceneRoot)) (Transformation|GetWorldLocation (Variables|/Game/MyContent/Characters/Blueprints/Spore2ScoreCharacter.Spore2ScoreCharacter_C|GetFollowCamera _asspore_2score_character))) false false))

(event Custom|DecreaseHealth
  (params (DecreaseAmount :type Float%20%28single-precision%29))
  ;[1 1 1] Update Health Property
  (bind _output_get (Variables|Health|SetHealth (Math|Float|Clamp(Float) (- (Variables|Health|GetHealth) DecreaseAmount) 0.0 (Variables|Health|GetMaxHealth))))
  (Variables|Health|SetIsHealthy (< _output_get 1e+02)))

(event Custom|Increase%20Nutrients_Event
  (params (amount :type Float%20%28single-precision%29))
  ;[1 1 1] Assign and register Increase Nutrients Message
  (CallFunction|IncreaseNutrients amount))

(event Custom|Grow
  (bind _staticmesh (Variables|Default|GetStaticMesh))
  (bind _returnvalue (Transformation|GetWorldScale _staticmesh))
  ;[1 1 1] Grow the plant
  (Transformation|SetWorldScale3D _staticmesh (Math|Vector|MakeVector (+ (.x _returnvalue) (Variables|Growth|GetBaseScaleFactor)) (+ (.y _returnvalue) (Variables|Growth|GetBaseScaleFactor)) (+ (.z _returnvalue) (Variables|Growth|GetHeightScaleFactor)))))

(event Custom|DeteriorateMessage_Event
  (params (isDeteriorating :type Boolean))
  ;[1 1 1] Assign and register Increase Nutrients Message
  (Variables|Health|SetIsDeteriorating isDeteriorating))

(event Custom|IncreaseHealth
  (params (HealthAmount :type Float%20%28single-precision%29))
  ;[1 1 1] Update Health Property
  (bind _output_get (Variables|Health|SetHealth (Math|Float|Clamp(Float) (+ (Variables|Health|GetHealth) HealthAmount) 0.0 (Variables|Health|GetMaxHealth))))
  (Variables|Health|SetIsHealthy (>= _output_get 1e+02)))

(event Custom|IncreaseNutrients
  (params (amount :type Float%20%28single-precision%29))
  ;[1 1 1] Update Nutrients Property
  (Variables|Nutrients|SetNutrients (+ (Variables|Nutrients|GetNutrients) amount))
  (if (> (Variables|Nutrients|GetNutrients) 0.0)
    (Variables|Nutrients|SetIsNutrientDepleted false)
    (if (>= (Variables|Nutrients|GetNutrients) 1e+02)
      (CallFunction|IncreaseHealth amount))
    (else
      (Variables|Nutrients|SetIsNutrientDepleted true))))

(event Custom|DecreaseNutrients
  (params (amount :type Float%20%28single-precision%29))
  ;[1 1 1] Update Nutrients Property
  (Variables|Nutrients|SetNutrients (- (Variables|Nutrients|GetNutrients) amount))
  (if (> (Variables|Nutrients|GetNutrients) 0.0)
    (Variables|Nutrients|SetIsNutrientDepleted false)
    (else
      (Variables|Nutrients|SetIsNutrientDepleted true)
      (CallFunction|DecreaseHealth amount))))

(event EventBeginPlay
  (Utilities|FlowControl|Sequence
    (:then_0
      ;[1 1 1] Create and assign Widget
      (bind _asgrowable_widget_bp (Utilities|Casting|CastToGrowableWidget_BP (UserInterface|GetUserWidgetObject (Variables|Default|GetWidget))))
      (bind _output_get (Variables|Widget|SetHealthWidget _asgrowable_widget_bp))
      (Variables|/Game/MyContent/Widgets/GrowableWidget_BP.GrowableWidget_BP_C|SetOwningActor _output_get self))
    (:then_1
      ;[1 1 1] Assign and register Increase Nutrients Message
      (EventDispatchers|BindEventtoIncreaseNutrientsMessage (delegate Custom|Increase%20Nutrients_Event))
      (EventDispatchers|BindEventtoDeteriorateMessage (delegate Custom|DeteriorateMessage_Event)))
    (:then_2
      ;[1 1 1] Set the timer for LifeCycle
      (Utilities|Time|SetTimerbyFunctionName 0 "LifeCycle" 1.0 true))))

(fn ConstructionScript)

(fn LifeCycle
  (Utilities|FlowControl|Sequence
    (:then_0
      ;[1 1 1] Set health status
      (if (>= (Variables|Health|GetHealth) 1e+02)
        (Variables|Health|SetIsHealthy true)
        (else
          (Variables|Health|SetIsHealthy false))))
    (:then_1
      ;[1 1 1] Decrease nutrients if deteriorating
      (if (Variables|Health|GetIsDeteriorating)
        (CallFunction|DecreaseNutrients 1.0)))
    (:then_2
      ;[1 1 1] Check Plant Health
      (if (<= (Variables|Health|GetHealth) 0.0)
        ;[1 1 1] Destroy Actor if no health
        (Actor|DestroyActor)
        (else
          ;[1 1 1] Plant is flourishing, GROW!
          (bind _isflourishing (CallFunction|IsFlourishing))
          (if _isflourishing
            (CallFunction|Grow)))))))

(fn IsFlourishing
  (return (and (>= (Variables|Health|GetHealth) 1e+02) (>= (Variables|Nutrients|GetNutrients) 1e+02))))