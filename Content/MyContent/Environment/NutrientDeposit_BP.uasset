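; NutrientDeposit_BP is a world nutrient deposit that feeds nearby biological actors until it runs out.
; It starts with a random store, and a one-second looping LifeCycle timer feeds non-flourishing BiologicalMaster_BP actors within its influence sphere, draining the store.
; The deposit destroys itself when a cycle finds it empty.
; A trigger shows or hides its widget for the player character, turning it toward the follow camera only on overlap begin and end.
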(event OnComponentBeginOverlap(TriggerWidget)
  (params (OverlappedComponent :type Primitive%20Component%20Object%20Reference) (OtherActor :type Actor%20Object%20Reference) (OtherComp :type Primitive%20Component%20Object%20Reference) (OtherBodyIndex :type Integer) (bFromSweep :type Boolean) (SweepResult :type Hit%20Result%20Structure%20%28by%20ref%29))
  (Utilities|Casting|CastToSpore2ScoreCharacter OtherActor)
  (CallFunction|RotatetoFacePlayer)
  (Rendering|SetVisibility (Variables|Default|GetWidget) true false))

(event OnComponentEndOverlap(TriggerWidget)
  (params (OverlappedComponent :type Primitive%20Component%20Object%20Reference) (OtherActor :type Actor%20Object%20Reference) (OtherComp :type Primitive%20Component%20Object%20Reference) (OtherBodyIndex :type Integer))
  (Utilities|Casting|CastToSpore2ScoreCharacter OtherActor)
  (CallFunction|RotatetoFacePlayer)
  (Rendering|SetVisibility (Variables|Default|GetWidget) false false))

(event Custom|RotateToFacePlayer
  ;[1 1 1] Rotate Health Widget to face Player
  (bind _asspore_2score_character (Utilities|Casting|CastToSpore2ScoreCharacter (Game|GetPlayerCharacter 0)))
  (Transformation|SetWorldRotation (Variables|Default|GetWidget) (Math|Rotator|FindLookatRotation (Transformation|GetWorldLocation (Variables|Default|GetDefaultSceneRoot)) (Transformation|GetWorldLocation (Variables|/Game/MyContent/Characters/Blueprints/Spore2ScoreCharacter.Spore2ScoreCharacter_C|GetFollowCamera _asspore_2score_character))) false false))

(event EventBeginPlay
  (Utilities|Time|SetTimerbyFunctionName 0 "LifeCycle" 1.0 true)
  (Variables|Default|SetNutrientStoreLevel (Math|Random|RandomIntegerinRange 50 1000))
  (bind _asnutrient_deposit_widget_bp (Utilities|Casting|CastToNutrientDepositWidget_BP (UserInterface|GetUserWidgetObject (Variables|Default|GetWidget))))
  (bind _output_get (Variables|Default|SetNutrientDepositWidget _asnutrient_deposit_widget_bp))
  (Variables|/Game/MyContent/Widgets/NutrientDepositWidget_BP.NutrientDepositWidget_BP_C|SetOwner _output_get self))

(fn ConstructionScript)

(fn LifeCycle
  (bind _nutrientconsumption (Variables|Default|GetNutrientConsumption))
  (if (> (Variables|Default|GetNutrientStoreLevel) 0)
    (for _array_element (Collision|GetOverlappingActors (Variables|Default|GetSphereOfNutrientInfluence) "/Game/MyContent/Environment/InteractableItems/Biological/BiologicalMaster_BP.BiologicalMaster_BP_C" :!class /Script/Engine.PrimitiveComponent)
      (bind _asbiological_master_bp (Utilities|Casting|CastToBiologicalMaster_BP _array_element))
      (bind _isflourishing (Default|IsFlourishing _asbiological_master_bp))
      (if (not _isflourishing)
        (Default|CallIncreaseNutrientsMessage _asbiological_master_bp _nutrientconsumption)
        (Variables|Default|SetNutrientStoreLevel (- (Variables|Default|GetNutrientStoreLevel) (Math|Float|Truncate _nutrientconsumption)))))
    (else
      (Actor|DestroyActor))))